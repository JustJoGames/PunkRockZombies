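; BP_Speaker is a speaker actor that switches to its punk-rock state when the third-person character touches its hit box.
; On overlap, the cube takes the M_SpeakerGood material and three effect flipbooks switch to FB_PunkRockSpeaker.
; It then calls the EDSpeakerBroken dispatcher and disables the hit box's collision, so the change happens only once.
; The GetHit function is an empty stub.
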(event OnComponentBeginOverlap(HitBox)
  (params (OverlappedComponent :type Primitive%20Component%20Object%20Reference) (OtherActor :type Actor%20Object%20Reference) (OtherComp :type Primitive%20Component%20Object%20Reference) (OtherBodyIndex :type Integer) (bFromSweep :type Boolean) (SweepResult :type Hit%20Result%20Structure%20%28by%20ref%29))
  (Utilities|Casting|CastToBP_ThirdPersonCharacter OtherActor)
  (Rendering|Material|SetMaterial (Variables|Default|GetCube) 0 "/Game/Materials/M_SpeakerGood.M_SpeakerGood")
  (Sprite|SetFlipbook (Variables|Default|GetEffects1) "/Game/Effects/FB_PunkRockSpeaker.FB_PunkRockSpeaker")
  (Sprite|SetFlipbook (Variables|Default|GetEffect_BrainRot) "/Game/Effects/FB_PunkRockSpeaker.FB_PunkRockSpeaker")
  (Sprite|SetFlipbook (Variables|Default|GetEffects2) "/Game/Effects/FB_PunkRockSpeaker.FB_PunkRockSpeaker")
  (Default|CallEDSpeakerBroken)
  (Collision|SetCollisionEnabled (Variables|Default|GetHitBox) "NoCollision"))

(fn ConstructionScript)

(fn GetHit)